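; BP_PlaeyrCharecter is the player character Blueprint, providing basic movement and mouse look.
; WalkForward and WalkRihgt axis inputs add movement along the forward and right vectors of the full control rotation.
; Mouse X and Mouse Y axes drive controller yaw and pitch directly, with no sensitivity scaling.
; Tick and the construction script are empty.
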(event `InputAxis|WalkForward`
  (params (AxisValue :type "Float (single-precision)"))
  ;[1 1 1] Передвижение
  (`self.AddMovementInput` (`KismetMathLibrary.GetForwardVector` (`self.GetControlRotation`)) AxisValue))

(event `InputAxis|WalkRihgt`
  (params (AxisValue :type "Float (single-precision)"))
  ;[1 1 1] Передвижение
  (`self.AddMovementInput` (`KismetMathLibrary.GetRightVector` (`self.GetControlRotation`)) AxisValue))

(event `InputAxis|Mouse X`
  (params (AxisValue :type "Float (single-precision)"))
  ;[1 1 1] Вращение персонажа
  (`self.AddControllerYawInput` AxisValue))

(event `InputAxis|Mouse Y`
  (params (AxisValue :type "Float (single-precision)"))
  ;[1 1 1] Вращение персонажа
  (`self.AddControllerPitchInput` AxisValue))

(fn `UserConstructionScript`)